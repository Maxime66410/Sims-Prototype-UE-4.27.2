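; RTS player camera pawn that provides axis-driven movement, boom zoom, rotation with clamped pitch, and optional screen-edge scrolling.
; Forward and right inputs follow actor rotation, while MouseMoveOnAxis pushes along fixed world axes when the cursor touches a viewport edge.
; Tick drives edge scrolling, and the TransformCamera input reuses it with larger vectors.
; Zoom, transform and rotate set distinct cursor icons, which a self-rearming timer restores.
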(event `self.ReceiveBeginPlay`
  ;[1 1 1] On Play
  (set `PlayerController.bShowMouseCursor` true (`GameplayStatics.GetPlayerController` 0))
  (`self.SetCursorMouse` 1)
  (`self.ResetCursor`))

(event `InputAxis|MoveCameraForward`
  (params (AxisValue :type "Float (single-precision)"))
  (bind (_returnvalue_x _returnvalue_y) (`KismetMathLibrary.BreakVector` (`KismetMathLibrary.GetForwardVector` (`self.K2_GetActorRotation`))))
  ;[1 1 1] Camera Movement
  (`self.AddMovementInput` (`KismetMathLibrary.MakeVector` _returnvalue_x _returnvalue_y) AxisValue))

(event `InputAxis|MoveCameraRight`
  (params (AxisValue :type "Float (single-precision)"))
  (bind (_returnvalue_x _returnvalue_y) (`KismetMathLibrary.BreakVector` (`KismetMathLibrary.GetRightVector` (`self.K2_GetActorRotation`))))
  ;[1 1 1] Camera Movement
  (`self.AddMovementInput` (`KismetMathLibrary.MakeVector` _returnvalue_x _returnvalue_y) AxisValue))

(event `InputAxis|CameraZoom`
  (params (AxisValue :type "Float (single-precision)"))
  (bind _boom (`self.Boom`))
  (bind _rangecameradistance (`self.RangeCameraDistance`))
  ;[1 1 1] Camera Zoom
  (if (!= AxisValue 0.0)
    (`self.SetCursorMouse` 12)
    (set `SpringArmComponent.TargetArmLength` (`KismetMathLibrary.FClamp` (+ (`SpringArmComponent.TargetArmLength` _boom) (* (* AxisValue -1.0) (* (`GameplayStatics.GetWorldDeltaSeconds`) (`self.ZoomSpeed`)))) (`|GetArrayItem` _rangecameradistance) (`|GetArrayItem` _rangecameradistance 1)) _boom)))

(event `self.ReceiveTick`
  (params (DeltaSeconds :type "Float (single-precision)"))
  (bind (_returnvalue_x _returnvalue_y) (`KismetMathLibrary.BreakVector2D` (`WidgetLayoutLibrary.GetViewportSize`)))
  ;[1 1 1] Camera Auto Movement
  (if (`self.useRTSMouseOnViewPort`)
    (bind _returnvalue (`WidgetLayoutLibrary.GetMousePositionOnViewport`))
    (`self.MouseMoveOnAxis` (`KismetMathLibrary.BreakVector2D` _returnvalue) _returnvalue_x (0.0 -1.0 0.0))
    (`self.MouseMoveOnAxis` (`.Y` (`KismetMathLibrary.BreakVector2D` _returnvalue)) _returnvalue_y (1.0 0.0 0.0))))

(event `InputAxis|TransformCamera`
  (params (AxisValue :type "Float (single-precision)"))
  ;[1 1 1] Transform Camera
  (if (!= AxisValue 0.0)
    (`self.MouseTransform`)
    (`self.SetCursorMouse` 10)))

(event `ResetCursor`
  ;[1 1 1] Reset Mouse Cursor Icon
  (`self.SetCursorMouse` 1)
  (`KismetSystemLibrary.K2_SetTimerDelegate` (delegate `ResetCursor`) 0.2))

(event `InputAxis|RotateCamera`
  (params (AxisValue :type "Float (single-precision)"))
  ;[1 1 1] Rotate Camera
  (if (!= AxisValue 0.0)
    (`self.MouseRotation`)
    (`self.SetCursorMouse` 11)))

(fn `MouseMoveOnAxis`
  (params (PositionOnAxis :type "Float (double-precision)") (AxisLength :type "Float (double-precision)") (Axis :type "Vector Structure"))
  (bind _returnvalue (- AxisLength PositionOnAxis))
  (if (< _returnvalue 1.0)
    (`self.AddMovementInput` Axis -1.0)
    (elif (> _returnvalue (- AxisLength 1.0))
      (`self.AddMovementInput` Axis))))

(fn `MouseRotation`
  (bind _defaultsceneroot (`self.DefaultSceneRoot`))
  (`SceneComponent.K2_SetRelativeRotation` _defaultsceneroot (`KismetMathLibrary.MakeRotator` 0.0 (`KismetMathLibrary.FClamp` (+ (.pitch (.rotation (`SceneComponent.GetSocketTransform` _defaultsceneroot "None" "RTS_World"))) (* (`self.GetInputAxisKeyValue`) 2.0)) -10.0 65.0) (+ (.yaw (.rotation (`SceneComponent.GetSocketTransform` _defaultsceneroot "None" "RTS_World"))) (* (`self.GetInputAxisKeyValue`) 2.0))) false false))

(fn `MouseTransform`
  (bind (_returnvalue_x _returnvalue_y) (`KismetMathLibrary.BreakVector2D` (`WidgetLayoutLibrary.GetViewportSize`)))
  (bind _returnvalue (`WidgetLayoutLibrary.GetMousePositionOnViewport`))
  (`self.MouseMoveOnAxis` (`KismetMathLibrary.BreakVector2D` _returnvalue) _returnvalue_x (0.0 -10.0 0.0))
  (`self.MouseMoveOnAxis` (`.Y` (`KismetMathLibrary.BreakVector2D` _returnvalue)) _returnvalue_y (10.0 0.0 0.0)))

(fn `SetCursorMouse`
  (params (IntI :type Byte))
  (set `PlayerController.CurrentMouseCursor` (cast `EMouseCursor` IntI) (`GameplayStatics.GetPlayerController` 0)))

(fn `UserConstructionScript`)